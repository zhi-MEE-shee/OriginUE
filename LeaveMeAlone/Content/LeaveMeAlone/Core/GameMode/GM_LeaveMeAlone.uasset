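; GM_LeaveMeAlone is a game mode Blueprint that runs the countdown for a LeaveMeAlone match.
; A looping one-second timer started on BeginPlay decrements GameTime until it reaches zero.
; It then clears the timer, shows the WBP_TimeOutCase widget and switches to UI-only input with a visible cursor.
; An IsAlive check leading to the same screen is left unconnected and never runs.
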(event Custom|CustomEvent
  (bind _returnvalue (Game|GetPlayerController 0))
  (bind _output_get (Variables|Default|SetGame%20Time (- (Variables|Default|GetGame%20Time) 1)))
  (if (== _output_get 0)
    (Utilities|Time|ClearandInvalidateTimerbyHandle (Variables|Default|GetGame%20Timer%20Handle))
    (bind _returnvalue_2 (UserInterface|CreateWidget "/Game/LeaveMeAlone/Widgets/TimeOutCase/WBP_TimeOutCase.WBP_TimeOutCase_C"))
    (UserInterface|Viewport|AddtoViewport _returnvalue_2 0)
    (Input|SetInputModeUIOnly _returnvalue 0 "DoNotLock" false)
    (Variables|/Script/Engine.PlayerController|SetbShowMouseCursor _returnvalue true)))

(event EventBeginPlay
  (bind _returnvalue (Utilities|Time|SetTimerbyEvent (delegate Custom|CustomEvent) 1.0 true))
  (Variables|Default|SetGame%20Timer%20Handle _returnvalue))

(event EventTick
  (params (DeltaSeconds :type Float%20%28single-precision%29)))

(fn ConstructionScript)